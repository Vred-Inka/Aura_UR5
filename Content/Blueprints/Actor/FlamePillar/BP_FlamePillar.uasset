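; BP_FlamePillar is a flame pillar actor that animates the intensity of its FireLight to vary the firelight.
; On BeginPlay it randomly picks one of two intensity timelines, and each picks again when finished, forming an endless randomized loop.
; Each timeline update passes its curve value to ScaleFlameIntencity, which multiplies it by BaseIntencity and applies it to the light.
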(event `StartTimeLine_1`
  (bind (_direction _flameintencity) (`Timeline|FlameIntencity_1` :!via `PlayFromStart`)
    (:`Update`
      (`self.ScaleFlameIntencity` _flameintencity))
    (:`Finished`
      (`self.Choose Timeline`))))

(event `self.ReceiveBeginPlay`
  (`self.Choose Timeline`))

(event `StartTimeline_2`
  (bind (_direction _flameintencity) (`Timeline|FlameIntencity_2` :!via `PlayFromStart`)
    (:`Update`
      (`self.ScaleFlameIntencity` _flameintencity))
    (:`Finished`
      (`self.Choose Timeline`))))

(event `Choose Timeline`
  (switch `int` (`KismetMathLibrary.RandomIntegerInRange` 0 1)
    (:`0`
      (`self.StartTimeLine_1`))
    (:`1`
      (`self.StartTimeline_2`))))

(fn `ScaleFlameIntencity`
  (params (Intencity :type "Float (double-precision)"))
  (`LightComponent.SetIntensity` (`self.FireLight`) (* Intencity (`self.BaseIntencity`))))

(fn `UserConstructionScript`)